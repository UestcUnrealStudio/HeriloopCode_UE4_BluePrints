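; Decorative actor that forms a slowly spinning ring of scattered star meshes.
; The construction script fills the Stars instanced mesh in concentric rows, using Sum angular steps around RadiusOfSelf, with random radial, planar and height jitter plus random rotation.
; Tick adds a small fixed local rotation each frame, independent of delta time.
; An InstanceStars helper graph also adds randomly rotated instances, but the construction script does not use it.
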(event EventBeginPlay)

(event Collision|EventActorBeginOverlap
  (params (OtherActor :type Actor%20Object%20Reference)))

(event EventTick
  (params (DeltaSeconds :type Float%20%28single-precision%29))
  (Transformation|AddActorLocalRotation self "0,0.020000, 0" false false))

(fn ConstructionScript
  (for _index (range 1 (Variables|Default|GetSum))
    (for _index_2 (range 1 (Variables|Default|GetRows))
      (Components|InstancedStaticMesh|AddInstance (Variables|Default|GetStars) (Math|Transform|MakeTransform (Math|Vector|MakeVector (+ (* (Math|Trig|Cos(Degrees) (* _index (/ 3.6e+02 (Math|Conversions|ToFloat(Integer) (Variables|Default|GetSum))))) (+ (+ (* _index_2 1.5e+02) (Variables|Default|GetRadiusOfSelf)) (Math|Random|RandomFloatinRange -2e+02 2e+02))) (Math|Random|RandomFloatinRange -5e+01 5e+01)) (+ (* (+ (+ (* _index_2 1.5e+02) (Variables|Default|GetRadiusOfSelf)) (Math|Random|RandomFloatinRange -2e+02 2e+02)) (Math|Trig|Sin(Degrees) (* _index (/ 3.6e+02 (Math|Conversions|ToFloat(Integer) (Variables|Default|GetSum)))))) (Math|Random|RandomFloatinRange -5e+01 5e+01)) (Math|Random|RandomFloatinRange -5e+02 5e+02)) (Math|Rotator|MakeRotator (Math|Random|RandomFloatinRange 0.0 3.6e+02) (Math|Random|RandomFloatinRange 0.0 3.6e+02) (Math|Random|RandomFloatinRange 0.0 3.6e+02)) "1,1,1")))))